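; BP_Console is a store console actor that players can use while nearby and that spawns ordered items.
; Its box overlap events set and clear CanUseConsole on the overlapping Player.
; SpawnOrderedItem looks up the item's class in the ItemLists map and spawns the requested amount at SpawnPoint, printing each spawned actor's name.
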(event OnComponentBeginOverlap(Box)
  (params (OverlappedComponent :type Primitive%20Component%20Object%20Reference) (OtherActor :type Actor%20Object%20Reference) (OtherComp :type Primitive%20Component%20Object%20Reference) (OtherBodyIndex :type Integer) (bFromSweep :type Boolean) (SweepResult :type Hit%20Result%20Structure%20%28by%20ref%29))
  (bind _asplayer (Utilities|Casting|CastToPlayer OtherActor))
  (Variables|/Game/Character/Player.Player_C|SetbCanUseConsole _asplayer true))

(event OnComponentEndOverlap(Box)
  (params (OverlappedComponent :type Primitive%20Component%20Object%20Reference) (OtherActor :type Actor%20Object%20Reference) (OtherComp :type Primitive%20Component%20Object%20Reference) (OtherBodyIndex :type Integer))
  (bind _asplayer (Utilities|Casting|CastToPlayer OtherActor))
  (Variables|/Game/Character/Player.Player_C|SetbCanUseConsole _asplayer false))

(event Custom|SpawnOrderedItem
  (params (Item :type String) (Amount :type String))
  (bind _itemlists (Variables|Default|GetItemLists))
  (bind (_value _returnvalue) (Utilities|Map|Find _itemlists Item))
  (if _returnvalue
    (for _index (range 1 (Math|Conversions|ToInteger(Byte) Amount))
      (bind _returnvalue_2 (Game|SpawnActorfromClass _value (Transformation|GetWorldTransform (Variables|Default|GetSpawnPoint)) "Undefined" "MultiplyWithRoot" 0 0))
      (Development|PrintString (Utilities|GetDisplayName _returnvalue_2)))))

(event EventBeginPlay)

(event Collision|EventActorBeginOverlap
  (params (OtherActor :type Actor%20Object%20Reference)))

(event EventTick
  (params (DeltaSeconds :type Float%20%28single-precision%29)))

(fn ConstructionScript)