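; BP_Creature is a moving creature actor in the Title folder that vanishes when it reaches a red light.
; Tick moves it along its local X axis at a Speed scaled by delta time.
; When its Box overlaps a BP_RedLight, it triggers that light's OnFlicker and hides its static mesh.
; Any end overlap shows the mesh again after a short delay, without checking the other actor's type.
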(event OnComponentBeginOverlap(Box)
  (params (OverlappedComponent :type Primitive%20Component%20Object%20Reference) (OtherActor :type Actor%20Object%20Reference) (OtherComp :type Primitive%20Component%20Object%20Reference) (OtherBodyIndex :type Integer) (bFromSweep :type Boolean) (SweepResult :type Hit%20Result%20Structure%20%28by%20ref%29))
  (bind _asbp_red_light (Utilities|Casting|CastToBP_RedLight OtherActor))
  (Default|OnFlicker _asbp_red_light)
  (Rendering|SetVisibility (Variables|Default|GetStaticMesh) false false))

(event OnComponentEndOverlap(Box)
  (params (OverlappedComponent :type Primitive%20Component%20Object%20Reference) (OtherActor :type Actor%20Object%20Reference) (OtherComp :type Primitive%20Component%20Object%20Reference) (OtherBodyIndex :type Integer))
  (Utilities|FlowControl|Delay 2.0)
  (Rendering|SetVisibility (Variables|Default|GetStaticMesh) true false))

(event EventBeginPlay)

(event EventTick
  (params (DeltaSeconds :type Float%20%28single-precision%29))
  (Transformation|AddActorLocalOffset (Math|Vector|MakeVector (* DeltaSeconds (Variables|Default|GetSpeed)) 0.0 0.0) false false))

(fn ConstructionScript)