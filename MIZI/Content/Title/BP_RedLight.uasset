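; BP_RedLight is a title-area light prop, pairing a static mesh with a point light, that flickers and then goes dark.
; OnFlicker applies a flicker material to two mesh slots and uses the same material as the point light's light function.
; After a short delay, it sets the light intensity to zero and switches those slots to black unlit material.
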(event Custom|OnFlicker
  (bind _staticmesh (Variables|Default|GetStaticMesh))
  (bind _staticmesh_2 (Variables|Default|GetStaticMesh))
  (Rendering|Material|SetMaterial _staticmesh 1 "/Game/Title/MI_Flicker.MI_Flicker")
  (Rendering|Material|SetMaterial _staticmesh 3 "/Game/Title/MI_Flicker.MI_Flicker")
  (Rendering|Components|Light|SetLightFunctionMaterial (Variables|Default|GetPointLight) "/Game/Title/MI_Flicker.MI_Flicker")
  (Utilities|FlowControl|Delay 2.0)
  (Rendering|Components|Light|SetIntensity (Variables|Default|GetPointLight) 0.0)
  (Rendering|Material|SetMaterial _staticmesh_2 1 "/Engine/EngineDebugMaterials/BlackUnlitMaterial.BlackUnlitMaterial")
  (Rendering|Material|SetMaterial _staticmesh_2 3 "/Engine/EngineDebugMaterials/BlackUnlitMaterial.BlackUnlitMaterial"))

(fn ConstructionScript)