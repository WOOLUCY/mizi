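; Rifle weapon that fires a hitscan shot for the player character.
; OnFire decrements the ammo count, then after a short delay plays camera shake, muzzle effect and sound.
; It traces from player 0's first-person camera along its forward vector, with debug drawing on.
; Impact particles, a randomly sized temporary bullet-hole decal and damage follow without checking whether the trace hit.
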(event Custom|OnFire
  (Math|Integer|DecrementInt (Variables|Default|GetCurBulletAmount)
    (:%20%20
      (Utilities|FlowControl|Delay 0.2)
      (Camera|PlayWorldCameraShake "/Game/Item/Weapon/Rifle/CS_RiffleFire.CS_RiffleFire_C" (Transformation|GetActorLocation) 0.0 5e+02)
      (Effects|SpawnEmitterAttached "/Game/StarterContent/Particles/P_Explosion.P_Explosion" (Variables|Default|GetStaticMeshComponent) "MuzzleSocket" "0, 0, 0" "0, 0, 0" "0.050000,0.050000,0.050000")
      (Audio|PlaySoundatLocation "/Game/StarterContent/Audio/Explosion01.Explosion01" (Transformation|GetActorLocation) "0, 0, 0" 1.0 1.0 0.0 0 0 0 0)
      (bind _asbasic_character (Utilities|Casting|CastToBasicCharacter (Game|GetPlayerCharacter 0)))
      (bind _outhit (Collision|LineTraceByChannel (Transformation|GetWorldLocation (Variables|/Script/MIZI.BasicCharacter|GetFirstPersonCamera _asbasic_character)) (+ (Transformation|GetWorldLocation (Variables|/Script/MIZI.BasicCharacter|GetFirstPersonCamera _asbasic_character)) (* (Math|Vector|GetForwardVector (Variables|/Script/MIZI.BasicCharacter|GetFirstPersonCamera _asbasic_character)) 3e+03)) "TraceTypeQuery1" false 0 "ForOneFrame"))
      (Effects|SpawnEmitteratLocation "/Game/Blueprint/Gimmick/Turret/PS_LaserHit.PS_LaserHit" (.Location (Collision|BreakHitResult _outhit)) (Math|Conversions|RotationFromXVector (.ImpactNormal (Collision|BreakHitResult _outhit))) "0.100000,0.100000,0.100000")
      (bind _returnvalue (Rendering|Decal|SpawnDecalatLocation "/Game/Item/Weapon/Rifle/Materials/M_BulletHole.M_BulletHole" (Math|Conversions|ToVector(Float) (Math|Random|RandomIntegerinRange 3 7)) (.Location (Collision|BreakHitResult _outhit)) (Math|Conversions|RotationFromXVector (.ImpactNormal (Collision|BreakHitResult _outhit))) 5.0))
      (Rendering|Components|Decal|SetFadeScreenSize _returnvalue 0.0)
      (Game|Damage|ApplyDamage (.HitActor (Collision|BreakHitResult _outhit)) (Variables|Default|GetRiffleDamage) 0 _asbasic_character))))

(event EventBeginPlay)

(event Collision|EventActorBeginOverlap
  (params (OtherActor :type Actor%20Object%20Reference)))

(event EventTick
  (params (DeltaSeconds :type Float%20%28single-precision%29)))

(fn ConstructionScript)