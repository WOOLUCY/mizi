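; BP_RifleBullet is a rifle ammo item that reloads the player's rifle when used.
; OnUsed plays the reload montage on player 0 and delays until one second before the montage's returned length.
; It then finds a BP_Rifle in the level with GetActorOfClass and adds a fixed bullet count to its current ammo, clamped to the rifle's maximum.
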(event Custom|OnUsed
  (bind _asplayer (Utilities|Casting|CastToPlayer (Game|Player|GetPlayerPawn 0)))
  (bind _returnvalue (Animation|PlayAnimMontage _asplayer "/Game/Character/Animation/RiffleAnimation/ANM_Reload.ANM_Reload" 1.0 "None"))
  (Utilities|FlowControl|Delay (- _returnvalue 1.0))
  (bind _returnvalue_2 (Actor|GetActorOfClass "/Game/Item/Weapon/Rifle/BP_Rifle.BP_Rifle_C"))
  (Variables|/Game/Item/Weapon/Rifle/BP_Rifle.BP_Rifle_C|SetCurBulletAmount _returnvalue_2 (Math|Integer|Clamp(Integer) (+ (Variables|/Game/Item/Weapon/Rifle/BP_Rifle.BP_Rifle_C|GetCurBulletAmount _returnvalue_2) 10) 0 (Variables|/Game/Item/Weapon/Rifle/BP_Rifle.BP_Rifle_C|GetMaxBulletAmount _returnvalue_2))))

(event EventBeginPlay)

(event Collision|EventActorBeginOverlap
  (params (OtherActor :type Actor%20Object%20Reference)))

(event EventTick
  (params (DeltaSeconds :type Float%20%28single-precision%29)))

(fn ConstructionScript)