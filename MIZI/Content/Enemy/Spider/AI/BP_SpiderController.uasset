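; BP_SpiderController is the AI controller for the spider enemy, running the BT_Spider behavior tree on BeginPlay.
; Its AIPerception update writes a sighted actor to the blackboard's TargetActor and the stimulus location to LastKnownLocation.
; Lost sight or any non-sight stimulus clears TargetActor, leaving LastKnownLocation untouched.
; The HandleSightSense function is an empty stub, with sight logic living directly in the event graph.
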(event OnTargetPerceptionUpdated(AIPerception)
  (params (Actor :type Actor%20Object%20Reference) (Stimulus :type AI%20Stimulus%20Structure))
  (bind (_age _expirationage _strength _stimuluslocation _receiverlocation _tag _bsuccessfullysensed) (Utilities|Struct|BreakAIStimulus Stimulus))
  (bind _returnvalue (Class|AIPerceptionSystem|GetSenseClassforStimulus Stimulus))
  (if (== _returnvalue "/Script/AIModule.AISense_Sight")
    (if _bsuccessfullysensed
      (AI|Components|Blackboard|SetValueasObject (AI|GetBlackboard 0) (Utilities|Name|MakeLiteralName "TargetActor") Actor)
      (AI|Components|Blackboard|SetValueasVector (AI|GetBlackboard 0) (Utilities|Name|MakeLiteralName "LastKnownLocation") _stimuluslocation)
      (else
        (AI|Components|Blackboard|SetValueasObject (AI|GetBlackboard 0) (Utilities|Name|MakeLiteralName "TargetActor") 0 :!label _label)))
    (else
      (goto _label))))

(event EventBeginPlay
  (AI|RunBehaviorTree "/Game/Enemy/Spider/AI/BT_Spider.BT_Spider"))

(fn ConstructionScript)

(fn HandleSightSense)