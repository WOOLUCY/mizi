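; BP_CameraMan is an enemy that takes a photo of the player, briefly flagging them with a screen flash.
; TakePhoto plays the camera animation and shutter sound, then waits a few seconds before showing the WBP_Flash widget.
; The player's IsDetecting flag is true only while the flash is on screen, then both are cleared.
; The file contains no trigger or visibility check for the photo.
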(event Custom|TakePhoto
  (Components|Animation|PlayAnimation (Variables|Default|GetCamera) "/Game/Enemy/CameraMan/Assets/Camera/camera_Anim_Armature_camera_moving_out_in.camera_Anim_Armature_camera_moving_out_in" false)
  (Audio|PlaySoundatLocation "/Game/Enemy/CameraMan/Assets/Audio/VINTAGE_CAMERA_SOUND_EFFECT.VINTAGE_CAMERA_SOUND_EFFECT" (Transformation|GetActorLocation) "0, 0, 0" 1.0 1.0 0.0 0 0 0 0)
  (bind _returnvalue (UserInterface|CreateWidget "/Game/Enemy/CameraMan/WBP_Flash.WBP_Flash_C"))
  (Utilities|FlowControl|Delay 2.8)
  (bind _asplayer (Utilities|Casting|CastToPlayer (Game|GetPlayerCharacter 0)))
  (Variables|/Game/Character/Player.Player_C|SetbIsDetecting _asplayer true)
  (UserInterface|Viewport|AddtoViewport _returnvalue 0)
  (Utilities|FlowControl|Delay 0.2)
  (Widget|RemovefromParent _returnvalue)
  (Variables|/Game/Character/Player.Player_C|SetbIsDetecting _asplayer false))

(fn ConstructionScript)