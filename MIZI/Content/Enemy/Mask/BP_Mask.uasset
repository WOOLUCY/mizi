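; BP_Mask is an enemy mask that constantly turns toward the player and awakens once it has been seen.
; Tick counts encounters, throttled by a delay, when the mesh was recently rendered and lies within the player's forward cone.
; An encounter activates it: the AI blackboard flag is set, mask materials swap to the character mesh, and a sound plays.
; Deactivate reverses this, while SetIsDetected writes render visibility to the blackboard and Attack is a stub.
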(event Custom|FacePlayer
  (Transformation|SetActorRotation (Math|Rotator|FindLookatRotation (Transformation|GetActorLocation) (Transformation|GetActorLocation (Game|GetPlayerCharacter 0)))))

(event Custom|SetIsDetected
  (bind _returnvalue (Utilities|Name|MakeLiteralName "IsDetected"))
  (bind _self self)
  (bind _returnvalue_2 (AI|GetAIController _self))
  (bind _returnvalue_3 (AI|GetBlackboard _returnvalue_2))
  (if (Class|PrimitiveComponent|WasRecentlyRendered (Variables|Character|GetMesh) 0.05)
    (AI|Components|Blackboard|SetValueasBool _returnvalue_3 _returnvalue false)
    (else
      (AI|Components|Blackboard|SetValueasBool _returnvalue_3 _returnvalue true))))

(event Custom|SetEncounterNum
  (bind _returnvalue (Game|GetPlayerCharacter 0))
  (if (Class|PrimitiveComponent|WasRecentlyRendered (Variables|Character|GetMesh) 0.05)
    (if (>= (Math|Vector|DotProduct (Math|Rotator|GetRotationXVector (Math|Rotator|FindLookatRotation (Transformation|GetActorLocation _returnvalue) (Transformation|GetActorLocation))) (Transformation|GetActorForwardVector _returnvalue)) 0.5)
      (Utilities|FlowControl|DoOnce false :!label _label
        (:Completed
          (bind _result (Math|Integer|IncrementInt (Variables|Default|GetEncounterNum))
            (:%20%20
              (Development|PrintString (Utilities|String|ToString(Integer) _result))
              (Utilities|FlowControl|Delay 4.0)
              (goto _label Reset))))))))

(event Custom|Activate
  (bind _sm_mask (Variables|Default|GetSM_Mask))
  (bind _sm_mask_2 (Variables|Default|GetSM_Mask))
  (if (not (ScalableFloat|GetValueasBool (AI|GetBlackboard (AI|GetAIController self)) (Utilities|Name|MakeLiteralName "IsActive")))
    (if (> (Variables|Default|GetEncounterNum) 0)
      (Utilities|FlowControl|DoOnce false
        (:Completed
          (AI|Components|Blackboard|SetValueasBool (AI|GetBlackboard (AI|GetAIController self)) (Utilities|Name|MakeLiteralName "IsActive") true)
          (Rendering|SetActorHiddenInGame false)
          (Rendering|Material|SetMaterial _sm_mask_2 1 "/Game/Enemy/Mask/M_Transparent.M_Transparent")
          (Rendering|Material|SetMaterial _sm_mask_2 0 "/Game/Enemy/Mask/M_Transparent.M_Transparent")
          (Rendering|Material|SetMaterial _sm_mask_2 2 "/Game/Enemy/Mask/M_Transparent.M_Transparent")
          (Rendering|Material|SetMaterial (Variables|Character|GetMesh) 0 "/Game/Enemy/Spider/CryingHead/CHmaterial.CHmaterial")
          (Audio|PlaySoundatLocation "/Game/Enemy/Mask/Assets/Audio/Active_Cue.Active_Cue" (Transformation|GetActorLocation) "0, 0, 0" 1.0 1.0 0.0 0 0 0 0)
          (Utilities|FlowControl|DoOnce false) ; enters at Reset
        )))))

(event Custom|Deactivate
  (bind _sm_mask (Variables|Default|GetSM_Mask))
  (bind _sm_mask_2 (Variables|Default|GetSM_Mask))
  (Utilities|FlowControl|DoOnce false
    (:Completed
      (AI|Components|Blackboard|SetValueasBool (AI|GetBlackboard (AI|GetAIController self)) (Utilities|Name|MakeLiteralName "IsActive") false)
      (Rendering|SetActorHiddenInGame true)
      (Rendering|Material|SetMaterial _sm_mask 0 "/Game/Enemy/Mask/Assets/Matcap_002.Matcap_002")
      (Rendering|Material|SetMaterial _sm_mask 1 "/Game/Enemy/Mask/Assets/Matcap_001.Matcap_001")
      (Rendering|Material|SetMaterial _sm_mask 2 "/Game/Enemy/Mask/Assets/Matcap_003.Matcap_003")
      (Rendering|Material|SetMaterial (Variables|Character|GetMesh) 0 "/Game/Enemy/Mask/M_Transparent.M_Transparent")
      (Variables|Default|SetEncounterNum 0)
      (Utilities|FlowControl|DoOnce false) ; enters at Reset
    )))

(event EventTick
  (params (DeltaSeconds :type Float%20%28single-precision%29))
  (CallFunction|FacePlayer)
  (CallFunction|SetEncounterNum)
  (CallFunction|Activate))

(fn ConstructionScript)

(fn Attack
  (return 0.0))