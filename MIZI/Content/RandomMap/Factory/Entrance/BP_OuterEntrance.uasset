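; Outer entrance actor that teleports the player into the factory dungeon of the random map.
; Each Tick it polls whether player 0 overlaps its Box and has CanInteract set, rather than using overlap events.
; When both hold, it sets the found DirectionalLight's intensity to zero, moves the player to DungeonLocation and DungeonRotation, and matches the controller's rotation.
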(event EventTick
  (params (DeltaSeconds :type Float%20%28single-precision%29))
  (bind _returnvalue (Game|GetPlayerCharacter 0))
  (if (Collision|IsOverlappingActor (Variables|Default|GetBox) _returnvalue :!class /Script/Engine.PrimitiveComponent)
    (bind _asplayer (Utilities|Casting|CastToPlayer _returnvalue))
    (if (Variables|/Game/Character/Player.Player_C|GetbCanInteract _asplayer)
      (bind _returnvalue_2 (Actor|GetActorOfClass "/Script/Engine.DirectionalLight"))
      (Rendering|Components|Light|SetIntensity (Variables|/Script/Engine.Light|GetLightComponent _returnvalue_2) 0.0)
      (Transformation|SetActorLocationAndRotation (Game|GetPlayerCharacter 0) (Variables|Default|GetDungeonLocation) (Variables|Default|GetDungeonRotation) false true)
      (Pawn|SetControlRotation (Game|GetPlayerController 0) (Variables|Default|GetDungeonRotation)))))

(fn ConstructionScript)