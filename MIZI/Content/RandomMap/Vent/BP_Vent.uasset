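; BP_Vent is a random-map vent that spawns random enemies from a class-to-count map, with GS_Basic as the required game state.
; SpawnRandomEnemy picks a random key, checks for a positive count, spawns at the Box transform and decrements the spawned class's count.
; The random pick is wired separately into check and spawn, so the classes can differ.
; A failed check only prints a message, without retrying.
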(event Custom|SpawnRandomEnemy
  (Utilities|Casting|CastToGS_Basic (Game|GetGameState))
  (bind _keys (Utilities|Map|Keys 0))
  (if (> (.Value (Utilities|Map|Find 0 (.OutItem (Utilities|Array|Random _keys)))) 0)
    (bind _returnvalue (Game|SpawnActorfromClass (.OutItem (Utilities|Array|Random _keys)) (Transformation|GetWorldTransform (Variables|Default|GetBox)) "Undefined" "MultiplyWithRoot" 0 0))
    (Utilities|Map|Add 0 (Utilities|GetClass _returnvalue) (- (.Value (Utilities|Map|Find 0 (Utilities|GetClass _returnvalue))) 1))
    (else
      (Development|PrintString "Enemy is not spawned" true true "(R=0.000000,G=0.660000,B=1.000000,A=1.000000)" 0.0))))

(fn ConstructionScript)