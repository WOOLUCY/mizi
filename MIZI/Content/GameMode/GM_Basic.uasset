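; GM_Basic is a game mode that covers the FactoryLevel map with a loading screen until the dungeon is complete.
; On BeginPlay in that level it switches the first player to UI-only input and shows a WBP_MapLoading widget.
; Tick polls DungeonComplete on BasicGameState and, every frame it is true, sets game-only input and hides the widget, without checking the level.
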(event EventBeginPlay
  (bind _returnvalue (Game|GetCurrentLevelName true))
  (if (Utilities|Enum|Equal(Enum) _returnvalue (Utilities|String|MakeLiteralString "FactoryLevel"))
    (Input|SetInputModeUIOnly (Game|GetPlayerController 0) 0 "DoNotLock" false)
    (bind _returnvalue_2 (UserInterface|CreateWidget "/Game/Character/Widget/WBP_MapLoading.WBP_MapLoading_C"))
    (bind _output_get (Variables|Default|SetLoadingScreen _returnvalue_2))
    (UserInterface|Viewport|AddtoViewport _output_get 0)))

(event EventTick
  (params (DeltaSeconds :type Float%20%28single-precision%29))
  (bind _asbasic_game_state (Utilities|Casting|CastToBasicGameState (Game|GetGameState)))
  (if (Variables|/Script/MIZI.BasicGameState|GetbDungeonComplete _asbasic_game_state)
    (Input|SetInputModeGameOnly (Game|GetPlayerController 0) false)
    (Variables|/Script/UMG.Widget|SetVisibility (Variables|Default|GetLoadingScreen) "Hidden")))

(fn ConstructionScript)