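; BP_Item is a pickable item actor configured by row name from DT_Pickable.
; Construction sets its mesh, price range, equip socket and item data, sizing a sphere to the mesh bounds plus padding.
; BeginPlay fills the name and price widget, rolling the displayed price separately from the stored Price.
; Scanning briefly shows the animated widget, while using any item toggles a spotlight with a flashlight sound.
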(event Custom|OnScanned
  (bind _widget (Variables|Default|GetWidget))
  (bind _returnvalue (UserInterface|GetWidget _widget))
  (Rendering|SetVisibility _widget true false)
  (bind _aswbp_item (Utilities|Casting|CastToWBP_Item _returnvalue))
  (UserInterface|Animation|PlayAnimation _returnvalue (Variables|/Game/Blueprint/Item/WBP_Item.WBP_Item_C|GetScanEffect _aswbp_item) 0.0 1 "Forward" 1.5 false)
  (Utilities|FlowControl|Delay 3.0)
  (Rendering|SetVisibility (Variables|Default|GetWidget) false false)
  (Widget|SetVisibility (Variables|/Game/Blueprint/Item/WBP_Item.WBP_Item_C|GetScanImage _aswbp_item) "Hidden"))

(event Custom|OnUsed
  (Audio|PlaySound2D "/Engine/VREditor/Sounds/UI/Flashlight_Switch.Flashlight_Switch" 1.0 1.0 0.0 0 0)
  (Utilities|FlowControl|FlipFlop
    (:A
      (Rendering|SetVisibility (Variables|Default|GetSpotLight) true false))
    (:B
      (Rendering|SetVisibility (Variables|Default|GetSpotLight) false false))))

(event EventBeginPlay
  (bind _minprice (Variables|Default|GetMinPrice))
  (bind _maxprice (Variables|Default|GetMaxPrice))
  (bind _returnvalue (Math|Random|RandomIntegerinRange _minprice _maxprice))
  (bind _aswbp_item (Utilities|Casting|CastToWBP_Item (UserInterface|GetWidget (Variables|Default|GetWidget))))
  (Variables|/Script/UMG.TextBlock|SetText (Variables|/Game/Blueprint/Item/WBP_Item.WBP_Item_C|GetItemName _aswbp_item) (Utilities|Text|ToText(Name) (Variables|Default|GetRowName)))
  (Variables|Default|SetPrice _returnvalue)
  (Variables|/Script/UMG.TextBlock|SetText (Variables|/Game/Blueprint/Item/WBP_Item.WBP_Item_C|GetItemPrice _aswbp_item) (Utilities|Text|ToText(Integer) _returnvalue)))

(fn ConstructionScript
  (bind _returnvalue (Utilities|GetDataTableRow "/Game/Blueprint/Item/DT_Pickable.DT_Pickable" (Variables|Default|GetRowName))
    (:then
      (Components|StaticMesh|SetStaticMesh (Variables|Default|GetStaticMesh) (.Mesh (Utilities|Struct|BreakPickable _returnvalue)))
      (Variables|Default|SetMinPrice (.MinPrice (Utilities|Struct|BreakPickable _returnvalue)))
      (Variables|Default|SetMaxPrice (.MaxPrice (Utilities|Struct|BreakPickable _returnvalue)))
      (Variables|Default|SetEquipSocketName (.EquipSocketName (Utilities|Struct|BreakPickable _returnvalue)))
      (Variables|Default|SetbUsed (.bUsed (Utilities|Struct|BreakPickable _returnvalue)))
      (Variables|Default|SetItemData _returnvalue)
      (Components|Sphere|SetSphereRadius (Variables|Default|GetSphere) (+ (.SphereRadius (Collision|GetComponentBounds (Variables|Default|GetStaticMesh))) 5e+01) true)
      (Utilities|Casting|CastToWBP_Item (UserInterface|GetWidget (Variables|Default|GetWidget))))))