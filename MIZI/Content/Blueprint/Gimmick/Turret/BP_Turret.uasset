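; Turret gimmick that sweeps between yaw limits by reversing its RotatingMovement rate, with a laser beam updated every tick from muzzle socket to player.
; When PawnSensing sees a pawn, it reveals the laser, yaws toward BasicCharacter targets and spawns a BP_Bullet after a short delay.
; A timer then hides the laser and runs a timeline easing back to the initial yaw.
; An Attack function damages the player but is not called here.
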(event OnSeePawn(PawnSensing)
  (params (Pawn :type Pawn%20Object%20Reference))
  (bind _returnvalue (Transformation|GetActorLocation Pawn))
  (bind _returnvalue_2 (Transformation|GetActorLocation))
  (Rendering|SetVisibility (Variables|Default|GetLaser) true false)
  (Utilities|Casting|CastToBasicCharacter Pawn)
  (Transformation|SetActorRotation (Math|Rotator|FindLookatRotation (Math|Vector|MakeVector (.x _returnvalue_2) (.y _returnvalue_2) (.z _returnvalue_2)) (Math|Vector|MakeVector (.x _returnvalue) (.y _returnvalue) (.z _returnvalue_2))))
  (Utilities|FlowControl|Delay 0.2)
  (Game|SpawnActorfromClass "/Game/Blueprint/Gimmick/Turret/BP_Bullet.BP_Bullet_C" (Transformation|GetSocketTransform (Variables|Default|GetTurret) "BulletSocket" "RTS_World") "AdjustIfPossibleButAlwaysSpawn" "MultiplyWithRoot" 0 0)
  (Utilities|Time|SetTimerbyEvent (delegate Custom|OnLoseSightOfPawn) 3.0))

(event Custom|OnLoseSightOfPawn
  (Rendering|SetVisibility (Variables|Default|GetLaser) false false)
  (bind _newtrack_0 (Timeline|Timeline PlayFromStart)
    (:Update
      (Transformation|SetActorRotation (Math|Rotator|MakeRotator 0.0 0.0 (Math|Float|Lerp (.yaw (Transformation|GetActorRotation)) (.yaw (Variables|Default|GetInitialRotation)) _newtrack_0))))))

(event EventTick
  (params (DeltaSeconds :type Float%20%28single-precision%29))
  (bind _returnvalue (Transformation|GetActorRotation))
  (bind _laser (Variables|Default|GetLaser))
  (bind _rotatingmovement (Variables|Default|GetRotatingMovement))
  (bind _initialrotation (Variables|Default|GetInitialRotation))
  (bind _returnvalue_2 (- (.yaw _returnvalue) (.yaw _initialrotation)))
  (Utilities|FlowControl|Sequence
    (:then_0
      (if (or (>= _returnvalue_2 (Variables|Default|GetMaxTargetRoationAngle)) (<= _returnvalue_2 (Variables|Default|GetMinTargetRoationAngle)))
        (Variables|/Script/Engine.RotatingMovementComponent|SetRotationRate _rotatingmovement (* (Variables|/Script/Engine.RotatingMovementComponent|GetRotationRate _rotatingmovement) -1.0))))
    (:then_1
      (Class|ParticleSystemComponent|SetBeamSourcePoint _laser 0 (Transformation|GetSocketLocation (Variables|Default|GetTurret) "BulletSocket"))
      (Class|ParticleSystemComponent|SetBeamEndPoint _laser 0 (Transformation|GetActorLocation (Game|GetPlayerCharacter 0))))))

(event EventBeginPlay
  (Variables|Default|SetInitialRotation (Transformation|GetActorRotation))
  (bind _returnvalue (Effects|SpawnEmitterAttached "/Game/Blueprint/Gimmick/Turret/PS_Laser.PS_Laser" (Variables|Default|GetTurret) "None"))
  (bind _output_get (Variables|Default|SetLaser _returnvalue))
  (Rendering|SetVisibility _output_get false false))

(fn ConstructionScript)

(fn Attack
  (Game|Damage|ApplyDamage (Game|GetPlayerCharacter 0) 2e+01 0 0)
  (return 0.0))