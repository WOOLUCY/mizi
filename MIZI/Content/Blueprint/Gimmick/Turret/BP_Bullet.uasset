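; BP_Bullet is a turret bullet that damages whatever actor its Box overlaps.
; On overlap it applies fixed damage, plays an impact sound, attaches a randomly sized, short-lived decal aligned to the sweep normal, then destroys itself.
; An Attack function that damages player 0 directly is not called here, and a laser-hit emitter spawn is left unconnected.
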(event OnComponentBeginOverlap(Box)
  (params (OverlappedComponent :type Primitive%20Component%20Object%20Reference) (OtherActor :type Actor%20Object%20Reference) (OtherComp :type Primitive%20Component%20Object%20Reference) (OtherBodyIndex :type Integer) (bFromSweep :type Boolean) (SweepResult :type Hit%20Result%20Structure%20%28by%20ref%29))
  (bind (_bblockinghit _binitialoverlap _time _distance _location _impactpoint _normal) (Collision|BreakHitResult SweepResult))
  (Game|Damage|ApplyDamage OtherActor 2e+01 0 0)
  (Audio|PlaySoundatLocation "/Game/StarterContent/Audio/Collapse01.Collapse01" _location "0, 0, 0" 1.0 1.0 0.0 0 0 0 0)
  (Class|GameplayStatics|SpawnDecalAttached 0 (Math|Conversions|ToVector(Float) (Math|Random|RandomIntegerinRange 3 7)) OtherComp "None" _location (Math|Conversions|RotationFromXVector _normal) "KeepWorldPosition" 1e+01)
  (Actor|DestroyActor))

(fn ConstructionScript)

(fn Attack
  (Game|Damage|ApplyDamage (Game|GetPlayerCharacter 0) 2e+01 0 0)
  (return 0.0))