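; BP_Door01 is a double door in the RandomMap folder that slides open when its OnOpen event fires.
; Its Box overlap sets the Player's CanOpenDoor flag and stores itself as OverlappedDoor; leaving clears only the flag.
; OnOpen prints a message and plays a timeline that moves both leaves apart along local X.
; The timeline float is applied as a cumulative per-update offset, and no closing logic exists.
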(event OnComponentBeginOverlap(Box)
  (params (OverlappedComponent :type Primitive%20Component%20Object%20Reference) (OtherActor :type Actor%20Object%20Reference) (OtherComp :type Primitive%20Component%20Object%20Reference) (OtherBodyIndex :type Integer) (bFromSweep :type Boolean) (SweepResult :type Hit%20Result%20Structure%20%28by%20ref%29))
  (bind _asplayer (Utilities|Casting|CastToPlayer OtherActor))
  (Variables|/Game/Character/Player.Player_C|SetbCanOpenDoor _asplayer true)
  (Variables|/Game/Character/Player.Player_C|SetOverlappedDoor _asplayer self))

(event OnComponentEndOverlap(Box)
  (params (OverlappedComponent :type Primitive%20Component%20Object%20Reference) (OtherActor :type Actor%20Object%20Reference) (OtherComp :type Primitive%20Component%20Object%20Reference) (OtherBodyIndex :type Integer))
  (bind _asplayer (Utilities|Casting|CastToPlayer OtherActor))
  (Variables|/Game/Character/Player.Player_C|SetbCanOpenDoor _asplayer false))

(event Custom|OnOpen
  (Development|PrintString "The Door is opening")
  (bind _float (Timeline|DoorOpenTimeline PlayFromStart)
    (:Update
      (Transformation|AddLocalOffset (Variables|Default|GetLeftDoor) (Math|Vector|MakeVector (* _float -1.0) 0.0 0.0) false false)
      (Transformation|AddLocalOffset (Variables|Default|GetRightDoor) (Math|Vector|MakeVector _float 0.0 0.0) false false))))

(fn ConstructionScript)