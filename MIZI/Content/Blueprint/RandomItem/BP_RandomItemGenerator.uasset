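; BP_RandomItemGenerator scatters copies of a configurable item class across a box area.
; Ten seconds after BeginPlay, it spawns ItemCount items at random points, always spawning regardless of collision.
; Each point offsets the Box's relative location by a random X and Y within its scaled extent and a fixed Z.
; X only covers the positive half because its minimum is multiplied by zero, while Y spans both sides.
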(event Custom|GetRandomLocationFromBox
  (bind _box (Variables|Default|GetBox))
  (bind _returnvalue (Components|Box|GetScaledBoxExtent _box))
  (Variables|Default|SetRandomLocation (+ (Variables|/Script/Engine.SceneComponent|GetRelativeLocation (Variables|Default|GetBox)) (Math|Vector|MakeVector (Math|Random|RandomFloatinRange (* (.x _returnvalue) -1.0 0.0) (.x _returnvalue)) (Math|Random|RandomFloatinRange (* (.y _returnvalue) -1.0) (.y _returnvalue)) 2e+01))))

(event EventBeginPlay
  (Utilities|FlowControl|Delay 1e+01)
  (for _index (range 0 (- (Variables|Default|GetItemCount) 1))
    (CallFunction|GetRandomLocationfromBox)
    (Game|SpawnActorfromClass (Variables|Default|GetSpawnableItem) (Math|Transform|MakeTransform (Variables|Default|GetRandomLocation) "0, 0, 0" "1.000000,1.000000,1.000000") "AlwaysSpawn" "MultiplyWithRoot" 0 0)))

(fn ConstructionScript)