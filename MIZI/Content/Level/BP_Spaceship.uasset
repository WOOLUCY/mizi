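; Spaceship actor that tracks the player and items aboard and carries out the departure to SpaceshipLevel.
; Tick opens the sliding door when the player is in the Box and CanInteract; timelines offset it, scaled by game time, and a delay triggers closing.
; Box overlaps set the player's IsInShip and maintain ItemsInShip as class, transform and price records.
; OnLeave waits, plays LS_Leave, raises the ship by timeline, then opens the level.
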(event OnComponentBeginOverlap(Box)
  (params (OverlappedComponent :type Primitive%20Component%20Object%20Reference) (OtherActor :type Actor%20Object%20Reference) (OtherComp :type Primitive%20Component%20Object%20Reference) (OtherBodyIndex :type Integer) (bFromSweep :type Boolean) (SweepResult :type Hit%20Result%20Structure%20%28by%20ref%29))
  (Utilities|FlowControl|Sequence
    (:then_0
      (bind _asplayer (Utilities|Casting|CastToPlayer OtherActor))
      (Variables|/Game/Character/Player.Player_C|SetbIsInShip _asplayer true))
    (:then_1
      (bind _asitem_base (Utilities|Casting|CastToItemBase OtherActor))
      (Utilities|Set|Add (Variables|Default|GetItemsInShip) (Utilities|Struct|MakeS_ItemSave (Utilities|GetClass _asitem_base) (Transformation|GetActorTransform _asitem_base) (Variables|/Script/MIZI.ItemBase|GetPrice _asitem_base))))))

(event OnComponentEndOverlap(Box)
  (params (OverlappedComponent :type Primitive%20Component%20Object%20Reference) (OtherActor :type Actor%20Object%20Reference) (OtherComp :type Primitive%20Component%20Object%20Reference) (OtherBodyIndex :type Integer))
  (Utilities|FlowControl|Sequence
    (:then_0
      (bind _asplayer (Utilities|Casting|CastToPlayer OtherActor))
      (Variables|/Game/Character/Player.Player_C|SetbIsInShip _asplayer false))
    (:then_1
      (bind _asitem_base (Utilities|Casting|CastToItemBase OtherActor))
      (Utilities|Set|Remove (Variables|Default|GetItemsInShip) (Utilities|Struct|MakeS_ItemSave (Utilities|GetClass _asitem_base) (Transformation|GetActorTransform _asitem_base) (Variables|/Script/MIZI.ItemBase|GetPrice _asitem_base))))))

(event Custom|OnLeave
  (Utilities|FlowControl|Delay 3.0)
  (bind _outactor (Sequencer|Player|CreateLevelSequencePlayer "/Game/Level/LevelSequence/LS_Leave.LS_Leave"))
  (Sequencer|Player|Play (Variables|/Script/LevelSequence.LevelSequenceActor|GetSequencePlayer _outactor) :!class /Script/MovieScene.MovieSceneSequencePlayer)
  (bind _newtrack_0 (Timeline|LeaveTimeline Play)
    (:Update
      (Transformation|AddActorLocalOffset (Math|Vector|MakeVector 0.0 0.0 (* _newtrack_0 1e+01)) false false))
    (:Finished
      (Game|OpenLevel(byName) "SpaceshipLevel"))))

(event Custom|CloseDoor
  (if (Variables|Default|GetbIsOpened)
    (bind _newtrack_0 (Timeline|Timeline PlayFromStart)
      (:Update
        (Transformation|AddLocalOffset (Variables|Default|GetSM_Door) (Math|Vector|MakeVector 0.0 (* _newtrack_0 (Utilities|Time|GetTimeSeconds) -3.0) 0.0) false false)
        (Variables|Default|SetbIsOpened false)))))

(event Custom|OpenDoor
  (if (not (Variables|Default|GetbIsOpened))
    (bind _newtrack_0 (Timeline|DoorTimeline PlayFromStart)
      (:Update
        (Transformation|AddLocalOffset (Variables|Default|GetSM_Door) (Math|Vector|MakeVector 0.0 (* _newtrack_0 (Utilities|Time|GetTimeSeconds) 3.0) 0.0) false false)
        (Variables|Default|SetbIsOpened true)
        (Utilities|FlowControl|Delay 3.0)
        (CallFunction|CloseDoor)))))

(event EventTick
  (params (DeltaSeconds :type Float%20%28single-precision%29))
  (bind _returnvalue (Game|GetPlayerCharacter 0))
  (if (Collision|IsOverlappingActor (Variables|Default|GetBox) _returnvalue :!class /Script/Engine.PrimitiveComponent)
    (bind _asplayer (Utilities|Casting|CastToPlayer _returnvalue))
    (if (Variables|/Game/Character/Player.Player_C|GetbCanInteract _asplayer)
      (CallFunction|OpenDoor))))

(event Collision|EventActorBeginOverlap
  (params (OtherActor :type Actor%20Object%20Reference)))

(event EventBeginPlay)

(fn ConstructionScript)